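; Player-controllable tank Blueprint that maps input to camera aiming, track throttle and firing.
; Aim axes yaw AzimuthGimbal and pitch CameraArm, while the Fire action calls Fire.
; LeftTrackThrottle sets TrackL's throttle, while RightTrackThrottle and the ForwardIntent press set TrackR's and then TrackL's.
; BeginPlay passes the Turret and Barrel components to SetTurretAndBarrelReference, with no turret movement logic in this graph.
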(event EventBeginPlay)

(event Collision|EventActorBeginOverlap
  (params (OtherActor :type Actor%20Object%20Reference)))

(event EventTick
  (params (DeltaSeconds :type Float%20%28single-precision%29)))

(event EventBeginPlay
  ;[1 1 1] Turret and Barrel Movement
  (Class|Tank|SetTurretandBarrelReference (Variables|Default|GetTurret) (Variables|Default|GetBarrel)))

(event Input|ActionEvents|InputActionFire
  (params (Key :type Key%20Structure :default "AnyKey"))
  ;[1 1 1] Camera Controls
  (:Pressed
    (Class|Tank|Fire)))

(event Input|ActionEvents|InputActionForwardIntent
  (params (Key :type Key%20Structure :default "AnyKey"))
  (bind _throttle (Variables|Default|Getthrottle))
  (:Pressed
    (Class|TankTreadComponent|SetThrottle (Variables|Default|GetTrackR) _throttle)
    (Class|TankTreadComponent|SetThrottle (Variables|Default|GetTrackL) _throttle)))

(event Input|AxisEvents|InputAxisAimAzimuth
  (params (AxisValue :type Float%20%28single-precision%29))
  ;[1 1 1] Camera Controls
  (Transformation|AddLocalRotation (Variables|Default|GetAzimuthGimbal) (Math|Rotator|MakeRotator 0.0 0.0 AxisValue) false false))

(event Input|AxisEvents|InputAxisAimElevation
  (params (AxisValue :type Float%20%28single-precision%29))
  ;[1 1 1] Camera Controls
  (Transformation|AddLocalRotation (Variables|Default|GetCameraArm) (Math|Rotator|MakeRotator 0.0 AxisValue 0.0) false false))

(event Input|AxisEvents|InputAxisLeftTrackThrottle
  (params (AxisValue :type Float%20%28single-precision%29))
  (Class|TankTreadComponent|SetThrottle (Variables|Default|GetTrackL) (Variables|Default|Getthrottle)))

(event Input|AxisEvents|InputAxisRightTrackThrottle
  (params (AxisValue :type Float%20%28single-precision%29))
  (bind _throttle (Variables|Default|Getthrottle))
  (Class|TankTreadComponent|SetThrottle (Variables|Default|GetTrackR) _throttle)
  (Class|TankTreadComponent|SetThrottle (Variables|Default|GetTrackL) _throttle))

(fn ConstructionScript)